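; BP_GameMode is a game mode that handles the end of a mission through its OnMissionCompleted event.
; It adds a WBP_GameOver widget to the viewport and removes all top-level WBP_ObjectiveInfo widgets.
; It then blends the instigating pawn's player camera over to the first BP_SpectatorViewpoint actor found in the level, using a cubic view-target blend.
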(event `self.OnMissionCompleted`
  (params (InstigatorPawn :type "Pawn Object Reference"))
  (`|ExecutionSequence`
    (:`then_0`
      (bind _returnvalue (`|CreateWidget` "/Game/UI/WBP_GameOver.WBP_GameOver_C"))
      (`UserWidget.AddToViewport` _returnvalue 0))
    (:`then_1`
      (bind _foundwidgets (`WidgetBlueprintLibrary.GetAllWidgetsOfClass` "/Game/UI/WBP_ObjectiveInfo.WBP_ObjectiveInfo_C"))
      (for _array_element _foundwidgets
        (`Widget.RemoveFromParent` _array_element)))
    (:`then_2`
      (bind _asplayer_controller (cast `PlayerController` (`Pawn.GetController` InstigatorPawn)))
      (bind _outactors (`GameplayStatics.GetAllActorsOfClass` "/Game/Blueprints/BP_SpectatorVIewpoint.BP_SpectatorViewpoint_C"))
      (`PlayerController.SetViewTargetWithBlend` _asplayer_controller (`|GetArrayItem` _outactors) 2.0 "VTBlend_Cubic" 0.0 false))))

(fn `UserConstructionScript`)